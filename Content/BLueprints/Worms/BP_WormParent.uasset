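; BP_WormParent is the parent Blueprint for AI-controlled worms drawn as sprites.
; On BeginPlay it casts its controller to AIC_Worms and stores itself in that controller's blackboard under the WormRef key.
; Each Tick it snaps the sprite to one of two fixed world rotations based on the sign of the capsule's yaw, so it flips with the facing direction.
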(event EventBeginPlay
  (bind _asaic_worms (Utilities|Casting|CastToAIC_Worms (AI|GetAIController 0)))
  (AI|Components|Blackboard|SetValueasObject (AI|GetBlackboard _asaic_worms) (Variables|Default|GetWormRef) self))

(event Collision|EventActorBeginOverlap
  (params (OtherActor :type Actor%20Object%20Reference)))

(event EventTick
  (params (DeltaSeconds :type Float%20%28single-precision%29))
  (bind _sprite (Variables|Default|GetSprite))
  (if (< (.yaw (Transformation|GetWorldRotation (Variables|Collision|GetCapsuleComponent))) 0.0)
    (Transformation|SetWorldRotation _sprite "0.000000,180.000000,90.000000" false false)
    (else
      (Transformation|SetWorldRotation _sprite "0.000000,-180.000000,-90.000000" false false))))

(fn ConstructionScript)