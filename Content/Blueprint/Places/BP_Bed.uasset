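; Bed place actor that tracks which of its four sleep spots are occupied by worms.
; BeginPlay caches the Targets child components and the exact class of a found BP_WormParent actor, used to filter overlaps.
; Each spot's begin overlap marks the matching OccupiedTargets index if the worm's Blackboard CanSleep is true.
; End overlap clears it without that check; both print French debug messages.
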(event OnComponentEndOverlap(SleepTarget3)
  (params (OverlappedComponent :type Primitive%20Component%20Object%20Reference) (OtherActor :type Actor%20Object%20Reference) (OtherComp :type Primitive%20Component%20Object%20Reference) (OtherBodyIndex :type Integer))
  (CallFunction|ClearOccupiedTargets OtherActor OverlappedComponent))

(event OnComponentBeginOverlap(SleepTarget)
  (params (OverlappedComponent :type Primitive%20Component%20Object%20Reference) (OtherActor :type Actor%20Object%20Reference) (OtherComp :type Primitive%20Component%20Object%20Reference) (OtherBodyIndex :type Integer) (bFromSweep :type Boolean) (SweepResult :type Hit%20Result%20Structure%20%28by%20ref%29))
  (CallFunction|SetOccupiedTargets OtherActor OverlappedComponent))

(event OnComponentEndOverlap(SleepTarget)
  (params (OverlappedComponent :type Primitive%20Component%20Object%20Reference) (OtherActor :type Actor%20Object%20Reference) (OtherComp :type Primitive%20Component%20Object%20Reference) (OtherBodyIndex :type Integer))
  (CallFunction|ClearOccupiedTargets OtherActor OverlappedComponent))

(event OnComponentEndOverlap(SleepTarget2)
  (params (OverlappedComponent :type Primitive%20Component%20Object%20Reference) (OtherActor :type Actor%20Object%20Reference) (OtherComp :type Primitive%20Component%20Object%20Reference) (OtherBodyIndex :type Integer))
  (CallFunction|ClearOccupiedTargets OtherActor OverlappedComponent))

(event OnComponentBeginOverlap(SleepTarget3)
  (params (OverlappedComponent :type Primitive%20Component%20Object%20Reference) (OtherActor :type Actor%20Object%20Reference) (OtherComp :type Primitive%20Component%20Object%20Reference) (OtherBodyIndex :type Integer) (bFromSweep :type Boolean) (SweepResult :type Hit%20Result%20Structure%20%28by%20ref%29))
  (CallFunction|SetOccupiedTargets OtherActor OverlappedComponent))

(event OnComponentEndOverlap(SleepTarget1)
  (params (OverlappedComponent :type Primitive%20Component%20Object%20Reference) (OtherActor :type Actor%20Object%20Reference) (OtherComp :type Primitive%20Component%20Object%20Reference) (OtherBodyIndex :type Integer))
  (CallFunction|ClearOccupiedTargets OtherActor OverlappedComponent))

(event OnComponentBeginOverlap(SleepTarget1)
  (params (OverlappedComponent :type Primitive%20Component%20Object%20Reference) (OtherActor :type Actor%20Object%20Reference) (OtherComp :type Primitive%20Component%20Object%20Reference) (OtherBodyIndex :type Integer) (bFromSweep :type Boolean) (SweepResult :type Hit%20Result%20Structure%20%28by%20ref%29))
  (CallFunction|SetOccupiedTargets OtherActor OverlappedComponent))

(event OnComponentBeginOverlap(SleepTarget2)
  (params (OverlappedComponent :type Primitive%20Component%20Object%20Reference) (OtherActor :type Actor%20Object%20Reference) (OtherComp :type Primitive%20Component%20Object%20Reference) (OtherBodyIndex :type Integer) (bFromSweep :type Boolean) (SweepResult :type Hit%20Result%20Structure%20%28by%20ref%29))
  (CallFunction|SetOccupiedTargets OtherActor OverlappedComponent))

(event EventBeginPlay
  (Variables|Default|SetBedTargets (Components|GetChildrenComponents (Variables|Default|GetTargets) true))
  (bind _returnvalue (Actor|GetActorOfClass "/Game/Blueprint/Worms/BP_WormParent.BP_WormParent_C"))
  (Variables|Default|SetWormClassRef (Utilities|GetClass _returnvalue)))

(fn ConstructionScript)

(fn SetOccupiedTargets
  (params (OverlapWorm :type Actor%20Object%20Reference) (OverlapBox :type Primitive%20Component%20Object%20Reference))
  (if (== (Utilities|GetClass OverlapWorm) (Variables|Default|GetWormClassRef))
    (if (ScalableFloat|GetValueasBool (AI|GetBlackboard OverlapWorm) (Variables|Default|GetCanSleep?))
      (for (_array_element _array_index) (Variables|Default|GetBedTargets)
        (if (== _array_element OverlapBox)
          (Utilities|Array|SetArrayElem (Variables|Default|GetOccupiedTargets) _array_index true)
          (Development|PrintString (Utilities|String|ToString(Text) (Utilities|Text|FormatText "J'ai set la target en occupée à l'index :  {##}" _array_index))))))))

(fn ClearOccupiedTargets
  (params (OverlapWorm :type Actor%20Object%20Reference) (OverlapBox :type Primitive%20Component%20Object%20Reference))
  (if (== (Utilities|GetClass OverlapWorm) (Variables|Default|GetWormClassRef))
    (if true
      (for (_array_element _array_index) (Variables|Default|GetBedTargets)
        (if (== _array_element OverlapBox)
          (Utilities|Array|SetArrayElem (Variables|Default|GetOccupiedTargets) _array_index false)
          (Development|PrintString (Utilities|String|ToString(Text) (Utilities|Text|FormatText "J'ai set la target en libre à l'index :  {##}" _array_index))))))))