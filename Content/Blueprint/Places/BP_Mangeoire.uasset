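; Feeding trough (mangeoire) for worms that tracks which of its four eating spots are occupied.
; On BeginPlay it caches the children of Targets and takes the exact class of the first BP_WormParent actor found for filtering overlaps.
; Overlap begin flags the matching index in OccupiedTargetsList if the worm's CanEat blackboard key is true.
; Overlap end frees it unconditionally for that class, and both print debug messages.
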(event OnComponentBeginOverlap(MangeoireTarget2)
  (params (OverlappedComponent :type Primitive%20Component%20Object%20Reference) (OtherActor :type Actor%20Object%20Reference) (OtherComp :type Primitive%20Component%20Object%20Reference) (OtherBodyIndex :type Integer) (bFromSweep :type Boolean) (SweepResult :type Hit%20Result%20Structure%20%28by%20ref%29))
  (CallFunction|SetOccupiedTargets OtherActor OverlappedComponent))

(event OnComponentBeginOverlap(MangeoireTarget3)
  (params (OverlappedComponent :type Primitive%20Component%20Object%20Reference) (OtherActor :type Actor%20Object%20Reference) (OtherComp :type Primitive%20Component%20Object%20Reference) (OtherBodyIndex :type Integer) (bFromSweep :type Boolean) (SweepResult :type Hit%20Result%20Structure%20%28by%20ref%29))
  (CallFunction|SetOccupiedTargets OtherActor OverlappedComponent))

(event OnComponentBeginOverlap(MangeoireTarget4)
  (params (OverlappedComponent :type Primitive%20Component%20Object%20Reference) (OtherActor :type Actor%20Object%20Reference) (OtherComp :type Primitive%20Component%20Object%20Reference) (OtherBodyIndex :type Integer) (bFromSweep :type Boolean) (SweepResult :type Hit%20Result%20Structure%20%28by%20ref%29))
  (CallFunction|SetOccupiedTargets OtherActor OverlappedComponent))

(event OnComponentBeginOverlap(MangeoireTarget1)
  (params (OverlappedComponent :type Primitive%20Component%20Object%20Reference) (OtherActor :type Actor%20Object%20Reference) (OtherComp :type Primitive%20Component%20Object%20Reference) (OtherBodyIndex :type Integer) (bFromSweep :type Boolean) (SweepResult :type Hit%20Result%20Structure%20%28by%20ref%29))
  (CallFunction|SetOccupiedTargets OtherActor OverlappedComponent))

(event OnComponentEndOverlap(MangeoireTarget1)
  (params (OverlappedComponent :type Primitive%20Component%20Object%20Reference) (OtherActor :type Actor%20Object%20Reference) (OtherComp :type Primitive%20Component%20Object%20Reference) (OtherBodyIndex :type Integer))
  (CallFunction|ClearOccupiedTargets OtherActor OverlappedComponent))

(event OnComponentEndOverlap(MangeoireTarget2)
  (params (OverlappedComponent :type Primitive%20Component%20Object%20Reference) (OtherActor :type Actor%20Object%20Reference) (OtherComp :type Primitive%20Component%20Object%20Reference) (OtherBodyIndex :type Integer))
  (CallFunction|ClearOccupiedTargets OtherActor OverlappedComponent))

(event OnComponentEndOverlap(MangeoireTarget3)
  (params (OverlappedComponent :type Primitive%20Component%20Object%20Reference) (OtherActor :type Actor%20Object%20Reference) (OtherComp :type Primitive%20Component%20Object%20Reference) (OtherBodyIndex :type Integer))
  (CallFunction|ClearOccupiedTargets OtherActor OverlappedComponent))

(event OnComponentEndOverlap(MangeoireTarget4)
  (params (OverlappedComponent :type Primitive%20Component%20Object%20Reference) (OtherActor :type Actor%20Object%20Reference) (OtherComp :type Primitive%20Component%20Object%20Reference) (OtherBodyIndex :type Integer))
  (CallFunction|ClearOccupiedTargets OtherActor OverlappedComponent))

(event EventBeginPlay
  (for _array_element (Components|GetChildrenComponents (Variables|Default|GetTargets) true)
    (Utilities|Array|Add (Variables|Default|GetMangeoireTargets) _array_element))
  (bind _returnvalue (Actor|GetActorOfClass "/Game/Blueprint/Worms/BP_WormParent.BP_WormParent_C"))
  (Variables|Default|SetWormClassRef (Utilities|GetClass _returnvalue)))

(event Collision|EventActorBeginOverlap
  (params (OtherActor :type Actor%20Object%20Reference)))

(event EventTick
  (params (DeltaSeconds :type Float%20%28single-precision%29)))

(fn ConstructionScript)

(fn SetOccupiedTargets
  (params (OverlapWorm :type Actor%20Object%20Reference) (OverlapBox :type Primitive%20Component%20Object%20Reference))
  (if (== (Utilities|GetClass OverlapWorm) (Variables|Default|GetWormClassRef))
    (if (ScalableFloat|GetValueasBool (AI|GetBlackboard OverlapWorm) (Variables|Default|GetCanEat?))
      (for (_array_element _array_index) (Variables|Default|GetMangeoireTargets)
        (if (== _array_element OverlapBox)
          (Utilities|Array|SetArrayElem (Variables|Default|GetOccupiedTargetsList) _array_index true)
          (Development|PrintString (Utilities|String|ToString(Text) (Utilities|Text|FormatText "J'ai set la target en occupée à l'index :  {##}" _array_index))))))))

(fn ClearOccupiedTargets
  (params (OverlapWorm :type Actor%20Object%20Reference) (OverlapBox :type Primitive%20Component%20Object%20Reference))
  (if (== (Utilities|GetClass OverlapWorm) (Variables|Default|GetWormClassRef))
    (if true
      (for (_array_element _array_index) (Variables|Default|GetMangeoireTargets)
        (if (== _array_element OverlapBox)
          (Utilities|Array|SetArrayElem (Variables|Default|GetOccupiedTargetsList) _array_index false)
          (Development|PrintString (Utilities|String|ToString(Text) (Utilities|Text|FormatText "J'ai set la target en libre à l'index :  {##}" _array_index))))))))