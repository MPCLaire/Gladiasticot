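; Player Blueprint for a worm-raising game: handles cursor selection, worm orders, the inventory and the switch to fights.
; BeginPlay gathers worms and creates the main HUD; an input toggles the inventory, which blocks world clicks while open.
; Clicking a worm shows its stats widget, while clicking feeder or bed sets Blackboard keys so its AI eats or sleeps.
; GoToFight switches camera, locks the inventory and copies GameMode's first fighter stats onto FighterWorm.
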(event Input|EnhancedActionEvents|EnhancedInputActionIA_Click
  (params (ActionValue :type Boolean) (ElapsedSeconds :type Float%20%28double-precision%29) (TriggeredSeconds :type Float%20%28double-precision%29) (InputAction :type Input%20Action%20Object%20Reference :default "/Game/Blueprint/Player/Inputs/IA_Click.IA_Click"))
  (bind _returnvalue (Game|GetPlayerController 0))
  (bind _hitresult (Game|Player|GetHitResultUnderCursorbyChannel _returnvalue "TraceTypeQuery1" true))
  (bind _hitactor (Collision|BreakHitResult _hitresult))
  (:Started
    (if (Variables|Default|GetCanClick?)
      (if (== (Utilities|GetClass _hitactor) (Variables|Default|GetWormParentClass))
        ;[0.008624 0.6094 0.5425 0.5] vérifier sur quoi on a cliqué et set la variable CurrentWorm
        (for (_array_element _array_index) (Variables|Default|GetWormList)
          (if (== (Utilities|Array|Get(acopy) (Variables|Default|GetWormList) _array_index) _hitactor)
            (Variables|Default|SetCurrentWormRef _array_element)))
        ;[0.07015 0.4439 0.7292 0.5] Quand on clique sur un ver, afficher ou enlever le widget
        (if (Utilities|IsValid (Variables|Default|GetWormWidgetRef))
          (Widget|RemovefromParent (Variables|Default|GetWormWidgetRef)))
        (bind _returnvalue_2 (UserInterface|CreateWidget "/Game/Widgets/WB_Worm.WB_Worm_C"))
        (bind _output_get (Variables|Default|SetWormWidgetRef _returnvalue_2))
        (UserInterface|Viewport|AddtoViewport _output_get 0)
        (Default|GetWormReference (Variables|Default|GetWormWidgetRef) (Variables|Default|GetCurrentWormRef))
        (Default|ShowStats (Variables|Default|GetWormWidgetRef))
        (Variables|/Game/Blueprint/Worms/BP_WormParent.BP_WormParent_C|SetWormWidgetRef (Variables|Default|GetCurrentWormRef) _output_get)
        (Default|SetWormName (Variables|Default|GetWormWidgetRef) (Variables|/Game/Blueprint/Worms/BP_WormParent.BP_WormParent_C|GetWormName (Variables|Default|GetCurrentWormRef)))
        (else
          ;[0.15 0.15 0.15 0.5] Faire aller manger
          (if (== _hitactor (Variables|Default|GetMangeoireRef))
            (if (Utilities|IsValid (Variables|Default|GetCurrentWormRef))
              (AI|Components|Blackboard|SetValueasBool (AI|GetBlackboard (Variables|Default|GetCurrentWormRef)) (Variables|Default|GetCanEat?) true)
              (AI|Components|Blackboard|SetValueasObject (AI|GetBlackboard (Variables|Default|GetCurrentWormRef)) (Variables|Default|GetMangeoire) (Variables|Default|GetMangeoireRef)))
            (else
              ;[0.147 0.15 0.05074 0.5] faire aller dormir
              (if (== _hitactor (Variables|Default|GetBedRef))
                (if (Utilities|IsValid (Variables|Default|GetCurrentWormRef))
                  (AI|Components|Blackboard|SetValueasBool (AI|GetBlackboard (Variables|Default|GetCurrentWormRef)) (Variables|Default|GetCanSleep?) true)
                  (AI|Components|Blackboard|SetValueasObject (AI|GetBlackboard (Variables|Default|GetCurrentWormRef)) (Variables|Default|GetBed) (Variables|Default|GetBedRef)))
                (else
                  ;[0.2778 0.1962 0.8385 0.5] Enlever le widget s'il est visible
                  (Variables|Default|SetCurrentWormRef 0)
                  (if (Utilities|IsValid (Variables|Default|GetWormWidgetRef))
                    (Widget|RemovefromParent (Variables|Default|GetWormWidgetRef))
                    (Variables|Default|SetWormWidgetRef 0)))))))))))

(event Input|EnhancedActionEvents|EnhancedInputActionIA_Inventory
  (params (ActionValue :type Boolean) (ElapsedSeconds :type Float%20%28double-precision%29) (TriggeredSeconds :type Float%20%28double-precision%29) (InputAction :type Input%20Action%20Object%20Reference :default "/Game/Blueprint/Player/Inputs/IA_Inventory.IA_Inventory"))
  ;[0.06027 0.15 0.06786 0.5] Ouvrir l'inventaire
  (:Started
    (if (Variables|Default|GetCanOpenInventory?)
      (bind _foundwidgets (Widget|GetAllWidgetsOfClass "/Game/Widgets/WB_Inventory.WB_Inventory_C" true))
      (Variables|Default|SetWBInventoryRef (Utilities|Array|Get(acopy) _foundwidgets))
      (if (Utilities|IsValid (Variables|Default|GetWBInventoryRef))
        (Widget|RemovefromParent (Variables|Default|GetWBInventoryRef) :!label _label)
        (Variables|Default|SetWBInventoryRef 0)
        (Variables|Default|SetCanClick? true)
        (elif (Utilities|IsValid (Variables|Default|GetWBInventoryRef))
          (goto _label)
          (else
            (bind _returnvalue (UserInterface|CreateWidget "/Game/Widgets/WB_Inventory.WB_Inventory_C"))
            (UserInterface|Viewport|AddtoViewport _returnvalue 0)
            (Variables|Default|SetWBInventoryRef _returnvalue)
            (Variables|Default|SetCanClick? false)
            (if (Variables|/Game/Widgets/WB_MainWidget.WB_MainWidget_C|GetShowDuel? (Variables|Default|GetMainWidgetRef))
              (Default|ShowNotification (Variables|/Game/Widgets/WB_Inventory.WB_Inventory_C|GetWB_Tab0 _returnvalue)))))))))

(event EventBeginPlay
  (bind _returnvalue (Game|GetPlayerController 0))
  (Variables|/Script/Engine.PlayerController|SetbShowMouseCursor _returnvalue true)
  (Input|SetInputModeGameandUI _returnvalue 0 "DoNotLock" true false)
  (Variables|/Script/Engine.PlayerController|SetbEnableClickEvents _returnvalue true)
  (bind _asbp_third_person_game_mode (Utilities|Casting|CastToBP_ThirdPersonGameMode (Game|GetGameMode)))
  (Variables|Default|SetGMRef _asbp_third_person_game_mode)
  (bind _outactors (Actor|GetAllActorsOfClass "/Game/Blueprint/Worms/BP_WormParent.BP_WormParent_C"))
  (for _array_element _outactors
    (Utilities|Array|Add (Variables|Default|GetWormList) _array_element))
  (bind _returnvalue_2 (UserInterface|CreateWidget "/Game/Widgets/WB_MainWidget.WB_MainWidget_C"))
  (bind _output_get (Variables|Default|SetMainWidgetRef _returnvalue_2))
  (UserInterface|Viewport|AddtoViewport _output_get 0))

(event EventControllerChanged
  (params (OldController :type Controller%20Object%20Reference) (NewController :type Controller%20Object%20Reference))
  ;[0.15 0.15 0.15 0.5] Add imput mapping
  (bind _asplayer_controller (Utilities|Casting|CastToPlayerController NewController))
  (Input|AddMappingContext (PlayerController|LocalPlayerSubsystems|GetEnhancedInputLocalPlayerSubsystem _asplayer_controller) "/Game/Blueprint/Player/Inputs/IMC_Player.IMC_Player" 0 "(bIgnoreAllPressedKeysUntilRelease=True,bForceImmediately=False,bNotifyUserSettings=False)"))

(fn ConstructionScript)

(fn GotoFight
  (bind _gmref (Variables|Default|GetGMRef))
  (bind _fighterwormslist (Variables|/Game/ThirdPerson/Blueprints/BP_ThirdPersonGameMode.BP_ThirdPersonGameMode_C|GetFighterWormsList _gmref))
  (bind _output (Utilities|Array|Get(acopy) _fighterwormslist))
  (Game|Player|SetViewTargetwithBlend (Game|GetPlayerController 0) (Variables|Default|GetFightCamera) 0.0 "VTBlend_Linear" 0.0 false)
  (Widget|RemovefromParent (Variables|Default|GetWBInventoryRef))
  (Variables|Default|SetCanOpenInventory? false)
  (Default|SetWormStats (Variables|Default|GetFighterWorm) (Variables|/Game/Blueprint/Worms/BP_WormParent.BP_WormParent_C|GetCurrentHealth _output) (Variables|/Game/Blueprint/Worms/BP_WormParent.BP_WormParent_C|GetMaxHealth _output) (Variables|/Game/Blueprint/Worms/BP_WormParent.BP_WormParent_C|GetLevel _output) (Variables|/Game/Blueprint/Worms/BP_WormParent.BP_WormParent_C|GetCurrentFatigue _output) (Variables|/Game/Blueprint/Worms/BP_WormParent.BP_WormParent_C|GetMaxFatigue _output) (Variables|/Game/Blueprint/Worms/BP_WormParent.BP_WormParent_C|GetCurrentXP _output) (Variables|/Game/Blueprint/Worms/BP_WormParent.BP_WormParent_C|GetMaxXP _output) (Variables|/Game/Blueprint/Worms/BP_WormParent.BP_WormParent_C|GetStrength _output) (Variables|/Game/Blueprint/Worms/BP_WormParent.BP_WormParent_C|GetDefense _output) (Variables|/Game/Blueprint/Worms/BP_WormParent.BP_WormParent_C|GetWormColor _output)))