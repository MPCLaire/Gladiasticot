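; BP_FighterWorm is a sprite-based fighter worm that holds its own health, level, fatigue, XP, strength and defense stats.
; SetWormStats copies the passed-in values into the worm's variables and tints the Sprite with the given color.
; The click event checks CanClickOnWorm but performs no action yet, and the construction script is empty.
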(event MouseInput|EventActorOnClicked
  (params (ButtonPressed :type Key%20Structure :default "None"))
  (if (Variables|Default|GetCanClickOnWorm?)
    _))

(fn ConstructionScript)

(fn SetWormStats
  (params (CurrentHealth :type Integer) (MaxHealth :type Integer) (Level :type Integer) (CurrentFatigue :type Integer) (MaxFatigue :type Integer) (CurrentXP :type Integer) (MaxXP :type Integer) (Strength :type Integer) (Defense :type Integer) (Color :type Color%20Structure))
  (Variables|Default|SetCurrentHealth CurrentHealth)
  (Variables|Default|SetMaxHealth MaxHealth)
  (Variables|Default|SetLevel Level)
  (Variables|Default|SetCurrentFatigue CurrentFatigue)
  (Variables|Default|SetMaxFatigue MaxFatigue)
  (Variables|Default|SetCurrentXP CurrentXP)
  (Variables|Default|SetMaxXP MaxXP)
  (Variables|Default|SetStrength Strength)
  (Variables|Default|SetDefense Defense)
  (Sprite|SetSpriteColor (Variables|Default|GetSprite) (Math|Conversions|ToLinearColor(Color) Color)))