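; Parent Blueprint for an AI worm with a randomly colored sprite and a hunger-then-health survival countdown.
; BeginPlay registers the worm in its Blackboard and starts a one-second hunger timer; at zero, a health timer takes over and leads to an empty Die function.
; Each drain updates the injected widget's bars when valid.
; Tick snaps the sprite between two rotations by capsule yaw sign to keep it facing the player.
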(event Custom|StartHealth
  ;[0.725 0 1 0.5] Perdre de la vie
  (Utilities|Time|SetTimerbyEvent (delegate Custom|DrainHealth) 1.0 true))

(event Custom|DrainHunger
  ;[0 0.3969 0.9656 0.5] Perdre de la faim
  (bind _result (Math|Integer|DecrementInt (Variables|Default|GetCurrentHunger))
    (:%20%20
      (if (Utilities|IsValid (Variables|Default|GetWormWidgetRef))
        (Default|SetHungerBar (Variables|Default|GetWormWidgetRef)))
      (if (== _result 0)
        (Utilities|Time|ClearandInvalidateTimerbyHandle (stale Custom|StartHunger _returnvalue))
        (CallFunction|StartHealth)))))

(event Custom|StartHunger
  ;[0 0.3969 0.9656 0.5] Perdre de la faim
  (bind _returnvalue (Utilities|Time|SetTimerbyEvent (delegate Custom|DrainHunger) 1.0 true)))

(event Custom|DrainHealth
  ;[0.725 0 1 0.5] Perdre de la vie
  (bind _result (Math|Integer|DecrementInt (Variables|Default|GetCurrentHealth))
    (:%20%20
      (if (Utilities|IsValid (Variables|Default|GetWormWidgetRef))
        (Default|SetHealthBar (Variables|Default|GetWormWidgetRef)))
      (if (== _result 0)
        (CallFunction|Die)))))

(event EventBeginPlay
  (bind _colorlist (Variables|Default|GetColorList))
  (AI|Components|Blackboard|SetValueasObject (AI|GetBlackboard 0) (Variables|Default|GetWormRef) self)
  (CallFunction|StartHunger)
  (Sprite|SetSpriteColor (Variables|Default|GetSprite) (Math|Conversions|ToLinearColor(Color) (Utilities|Array|Get(acopy) _colorlist (Math|Random|RandomIntegerinRange 0 (- (Utilities|Array|Length _colorlist) 1))))))

(event EventTick
  (params (DeltaSeconds :type Float%20%28single-precision%29))
  (bind _sprite (Variables|Default|GetSprite))
  ;[0.15 0.1198 0.06121] fixe la rotation du sprite pour qu'il soit toujours face au joueur
  (if (< (.yaw (Transformation|GetWorldRotation (Variables|Default|GetCapsuleComponent))) 0.0)
    (Transformation|SetWorldRotation _sprite "0.000000,-90.000000,90.000000" false false)
    (else
      (Transformation|SetWorldRotation _sprite "0.000000,90.000000,-90.000000" false false))))

(fn ConstructionScript)

(fn Die)

(fn GetWidgetReference
  (params (WidgetRef :type WB%20Worm%20Object%20Reference))
  (Variables|Default|SetWormWidgetRef WidgetRef))